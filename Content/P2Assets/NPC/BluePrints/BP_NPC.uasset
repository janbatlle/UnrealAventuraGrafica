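; NPC Blueprint that shows a repeatable sequence of English dialogue lines on screen.
; Each Talk event advances TalkIndex and writes the next DialogueENG entry into a Dialogue widget, creating it if needed.
; Past the last line it removes the widget, resets the index and sets CanMove to false on the BP_BaseCharacter cached by the TriggerZone overlap.
; The DialogueESP variable is unused.
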(event `/Game/P2Assets/NPC/BluePrints/BP_Dialogue.Talk`
  ; Array de dialogos, se repiten
  (`/Engine/EditorBlueprintResources/StandardMacros.IncrementInt` (`self.talkIndex`)
    (:`  `
      (if (< (`self.talkIndex`) (`KismetArrayLibrary.Array_Length` (`self.dialogueENG`)))
        (`self.UI`
          (:`then`
            _)
          (:`else`
            (bind _returnvalue (`|CreateWidget` "/Game/P2Assets/NPC/BluePrints/Dialogue.Dialogue_C" (`GameplayStatics.GetPlayerController` 0)))
            (bind _output_get (set `self.UI` _returnvalue))
            (`UserWidget.AddToViewport` _output_get 0)))
        (`TextBlock.SetText` (`/Game/P2Assets/NPC/BluePrints/Dialogue.TalkText` (`self.UI`)) (`KismetTextLibrary.Conv_StringToText` (`|GetArrayItem` (`self.dialogueENG`) (`self.talkIndex`))))
        (else
          (`Widget.RemoveFromParent` (`self.UI`))
          (set `self.talkIndex` -1)
          (set `self.UI` null)
          (set `/Game/PlayerCharater/BluePrints/BP_BaseCharacter.CanMove?` false (`self.As BP Base Character`)))))))

(event `self.Trigger Zone.OnComponentBeginOverlap`
  (params (OverlappedComponent :type "PrimitiveComponent Object Reference") (OtherActor :type "Actor Object Reference") (OtherComp :type "PrimitiveComponent Object Reference") (OtherBodyIndex :type Integer) (bFromSweep :type Boolean) (SweepResult :type "HitResult Structure (by ref)"))
  (bind _asbp_base_character (cast `/Game/PlayerCharater/BluePrints/BP_BaseCharacter` OtherActor))
  (set `self.As BP Base Character` _asbp_base_character))

(fn `UserConstructionScript`)